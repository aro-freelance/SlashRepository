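; BP_SlashCharacter is a character Blueprint that keeps motion warping aligned to its combat target.
; Every Tick it calls UpdateMotionWarp, which, while CombatTarget is valid, feeds computed translation and rotation locations into the named TranslationTarget and RotationTarget warp targets.
; The target math comes from getter functions defined outside this graph.
; An unlinked sword attack montage snippet remains in the event graph and never runs.
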(event Input|EnhancedActionEvents|EnhancedInputActionIA_Attack
  (params (ActionValue :type Boolean) (ElapsedSeconds :type Float%20%28double-precision%29) (TriggeredSeconds :type Float%20%28double-precision%29) (InputAction :type Input%20Action%20Object%20Reference :default "/Game/Blueprints/Characters/Input/IA_Attack.IA_Attack"))
  ;[1 0.2052 0.2052] Unlinked: Attack Montage in Blueprints
)

(event EventBeginPlay)

(event Collision|EventActorBeginOverlap
  (params (OtherActor :type Actor%20Object%20Reference)))

(event EventTick
  (params (DeltaSeconds :type Float%20%28single-precision%29))
  (CallFunction|UpdateMotionWarp))

(fn ConstructionScript)

(fn UpdateMotionWarp
  (Variables|Default|GetCombatTarget
    (:then
      (bind _returnvalue (Class|BaseCharacter|GetTranslationWarpTarget))
      (Class|MotionWarpingComponent|AddorUpdateWarpTargetfromLocation (Variables|Default|GetMotionWarping) "TranslationTarget" _returnvalue)
      (bind _returnvalue_2 (Class|BaseCharacter|GetRotationWarpTarget))
      (Class|MotionWarpingComponent|AddorUpdateWarpTargetfromLocation (Variables|Default|GetMotionWarping) "RotationTarget" _returnvalue_2))
    (:else)))