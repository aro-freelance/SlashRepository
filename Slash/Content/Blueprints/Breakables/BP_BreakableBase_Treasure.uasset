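; Base Blueprint for a Chaos Geometry Collection breakable, apparently a treasure pot, layered on a native C++ parent.
; GetHit and unhit Chaos breaks both route through HandleHit, which flags the hit, plays the pot-break sound and calls the parent GetHit.
; The HasBeenHit flag stops break events from repeating that handling.
; On breaking, the actor sets a short lifespan and its capsule ignores pawns.
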(event OnChaosBreakEvent(GeometryCollection)
  (params (BreakEvent :type Chaos%20Break%20Event%20Structure%20%28by%20ref%29))
  (bind _returnvalue (Transformation|GetActorLocation))
  (if (Variables|Default|GetHasBeenHit)
    _
    (else
      (CallFunction|HandleHit _returnvalue _returnvalue)))
  (Actor|SetLifeSpan 2.0)
  (Collision|SetCollisionResponsetoChannel (Variables|Default|GetCapsule) "ECC_Pawn" "ECR_Ignore"))

(event EventBeginPlay)

(event Collision|EventActorBeginOverlap
  (params (OtherActor :type Actor%20Object%20Reference)))

(event EventTick
  (params (DeltaSeconds :type Float%20%28single-precision%29)))

(event EventGetHit
  (params (ImpactPoint :type Vector%20%28by%20ref%29 :default "0, 0, 0") (DamagerDealer :type Character%20Object%20Reference) (Weapon :type Weapon%20Object%20Reference))
  (CallFunction|HandleHit ImpactPoint ImpactPoint))

(fn ConstructionScript)

(fn HandleHit
  (params (ImpactPoint :type Vector%20%28by%20ref%29) (Location :type Vector))
  (Variables|Default|SetHasBeenHit true)
  (Audio|PlaySoundatLocation "/Game/Audio/MetaSounds/SFX_PotBreak.SFX_PotBreak" Location "0, 0, 0" 1.0 1.0 0.0 0 0 0 0)
  ;[0.9993 1 0.6612] Call the C++ Version. i.e Super
  (|CallParentFunction ImpactPoint 0 0))