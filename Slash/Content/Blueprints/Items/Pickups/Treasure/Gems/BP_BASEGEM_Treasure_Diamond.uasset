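; Diamond gem treasure pickup Blueprint that extends a parent class with a raised, spinning presentation.
; On BeginPlay it runs the parent logic, then moves the actor to 30 units above the item mesh's world position.
; Each Tick it runs the parent logic and adds yaw rotation from ZRotation scaled by delta time, giving a frame-rate-independent spin.
; The construction script only calls the parent.
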(event EventBeginPlay
  (bind _itemmesh (Variables|Default|GetItemMesh))
  (bind _returnvalue (Transformation|GetWorldLocation _itemmesh))
  (|CallParentFunction)
  (Transformation|SetActorLocation (Math|Vector|MakeVector (.x _returnvalue) (.y _returnvalue) (+ (.z _returnvalue) 3e+01)) false false))

(event EventTick
  (params (DeltaSeconds :type Float%20%28single-precision%29))
  (|CallParentFunction DeltaSeconds)
  (Class|Actor|AddActorWorldRotation (Math|Rotator|MakeRotator 0.0 0.0 (* DeltaSeconds (Variables|Default|GetZRotation)))))

(fn ConstructionScript
  (|CallParentFunction))