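; Base enemy Blueprint that patrols, chases a combat target and returns to its spawn point when hurt out of combat.
; BeginPlay saves a spawn marker and spawns a socket-attached weapon by weapon type, with matching attack montage.
; Tick sets speed and movement, picking new patrol goals when stationary, either random navigable points or array entries (random, looping, ping-pong).
; Blueprint aggro bindings are disconnected, noted as handled in C++.
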(event EventBeginPlay
  (CallFunction|SetWeapon)
  (CallFunction|InitializeMovementGoal)
  (Utilities|FlowControl|Delay 2.0)
  (Variables|Default|SetIsLoading false))

(event Collision|EventActorBeginOverlap
  (params (OtherActor :type Actor%20Object%20Reference)))

(event EventTick
  (params (DeltaSeconds :type Float%20%28single-precision%29))
  ;[1 1 1] Combat Movement
  (if (Variables|Default|GetIsInCombat)
    (Variables|Default|SetIsChangingDirection false)
    (Variables|/Script/Engine.CharacterMovementComponent|SetMaxWalkSpeed (Variables|Character|GetCharacterMovement) 4e+02)
    (CallFunction|PursuePlayerifinCombat)
    (else
      ;[1 1 1] Not in Combat, Patrol Speed
      (Variables|/Script/Engine.CharacterMovementComponent|SetMaxWalkSpeed (Variables|Character|GetCharacterMovement) 2e+02)
      ;[1 1 1] If Out of Combat and less than 100% HP, return to spawn
      (if (Variables|Default|GetIsReturning)
        (CallFunction|MovetoStartingLocation)
        (else
          ;[1 1 1] Pause While Changing Movement Goal Location
          (if (Variables|Default|GetIsChangingDirection)
            (Utilities|FlowControl|Delay (Variables|Default|GetStationaryDelayTime))
            (Variables|Default|SetIsChangingDirection false)
            (CallFunction|IdleMovement)
            (else
              ;[1 1 1] IF out of Combat without Full HP, Start Returning to Spawn and Regening
              (if (< (Variables|Default|GetHP) (Variables|Default|GetMaxHP))
                (Variables|Default|SetIsReturning true)
                (Variables|Default|SetIsRegening true)
                (Utilities|FlowControl|Delay (Variables|Default|GetStationaryDelayTime))
                (else
                  ;[1 1 1] Patrol
                  (CallFunction|IdleMovement)
                  ;[1 1 1] If Stationary, Start Changing Direction
                  (CallFunction|IfStationary,ChangeMovementGoal))))))))))

(fn ConstructionScript)

(fn PursuePlayerifinCombat
  (AI|Navigation|MovetoLocation (AI|GetAIController self) (Transformation|GetActorLocation (Variables|Default|GetCombatTarget)) -1.0 true true false true 0))

(fn IdleMovement
  ;[1 1 1] Store Location
  (Variables|Default|SetLocation%20Last%20TIck (Transformation|GetActorLocation))
  (Variables|Default|GetMovement%20Goal
    (:then
      ;[1 1 1] Move to Goal
      (AI|Navigation|SimpleMovetoActor (AI|GetAIController self) (Variables|Default|GetMovement%20Goal))
      ;[1 1 1] If Goal Reached, TODO: Add logic if reaching goal does something.  new goal will be set when stationary (don't set it here)
      (if (Utilities|Operators|EqualEqual (Transformation|GetActorLocation) (Transformation|GetActorLocation (Variables|Default|GetMovement%20Goal)) 5e+01)
        (if (Variables|Default|GetIsReturning)
          (Variables|Default|SetCounter_PatrolArray 0)
          (Variables|Default|SetIsChangingDirection true)
          (Variables|Default|SetIsReturning false))))
    (:else
      (CallFunction|SetNewMovementGoal))))

(fn SetNewMovementGoal
  (bind _arrayofpatrolgoals (Variables|Default|GetArrayOfPatrolGoals))
  (bind _returnvalue (Utilities|Array|LastIndex _arrayofpatrolgoals))
  ;[1 1 1] Patrol: Full Random
  (if (Utilities|Enum|Equal(Enum) (Variables|Default|GetPatrolType) "EPT_FullRandom")
    (Variables|Default|GetMovement%20Goal
      (:then
        _)
      (:else
        ;[1 1 1] Make Actor to use for Random Movement
        (bind _returnvalue_2 (Game|SpawnActorfromClass "/Game/Blueprints/BP_MovementGoalActor.BP_MovementGoalActor_C" (Transformation|GetActorTransform) "Undefined" 0 0))
        (Variables|Default|SetMovement%20Goal _returnvalue_2)))
    (bind _randomlocation (Class|NavigationSystemV1|GetRandomLocationinNavigableRadius (Transformation|GetActorLocation) 3e+03 0 0))
    (Transformation|SetActorLocation (Variables|Default|GetMovement%20Goal) _randomlocation false false)
    (else
      ;[1 1 1] Check the Array of Goals
      (if (> (Utilities|Array|Length (Variables|Default|GetArrayOfPatrolGoals)) 0)
        ;[1 1 1] Patrol: Random in Set
        (if (Utilities|Enum|Equal(Enum) (Variables|Default|GetPatrolType) "EPT_RandomInSet")
          (Variables|Default|SetMovement%20Goal (.OutItem (Utilities|Array|Random (Variables|Default|GetArrayOfPatrolGoals))))
          (else
            ;[1 1 1] Patrol: Goals in Order in Set. Loop back to Array[0] when end is reached.
            (if (Utilities|Enum|Equal(Enum) (Variables|Default|GetPatrolType) "EPT_SetOrderLoopEnd")
              (Variables|Default|SetMovement%20Goal (Utilities|Array|Get(acopy) (Variables|Default|GetArrayOfPatrolGoals) (Variables|Default|GetCounter_PatrolArray)))
              (if (< (Variables|Default|GetCounter_PatrolArray) (Utilities|Array|LastIndex (Variables|Default|GetArrayOfPatrolGoals)))
                (Variables|Default|SetCounter_PatrolArray (+ (Variables|Default|GetCounter_PatrolArray) 1))
                (else
                  (Variables|Default|SetCounter_PatrolArray 0)))
              (else
                ;[1 1 1] Patrol: Goals in Order in Set. Reverse when end is reached. (Array[length-1])
                (if (Utilities|Enum|Equal(Enum) (Variables|Default|GetPatrolType) "EPT_SetOrderReverseEnd")
                  (Variables|Default|SetMovement%20Goal (Utilities|Array|Get(acopy) (Variables|Default|GetArrayOfPatrolGoals) (Variables|Default|GetCounter_PatrolArray)))
                  (Development|PrintString (Utilities|GetDisplayName (Variables|Default|GetMovement%20Goal)) true true "(R=0.000000,G=0.660000,B=1.000000,A=1.000000)" 1e+01)
                  (if (Variables|Default|GetIsReversePatrol)
                    ;;[1 1 1] Reverse Counter Incrementer
                    (if (== (Variables|Default|GetCounter_PatrolArray) 0)
                      (Variables|Default|SetIsReversePatrol false)
                      (Variables|Default|SetCounter_PatrolArray 1)
                      (else
                        (Variables|Default|SetCounter_PatrolArray (- (Variables|Default|GetCounter_PatrolArray) 1))))
                    (else
                      ;;[1 1 1] Counter Incrementer
                      (if (< (Variables|Default|GetCounter_PatrolArray) _returnvalue)
                        (Variables|Default|SetCounter_PatrolArray (+ (Variables|Default|GetCounter_PatrolArray) 1))
                        (else
                          (Variables|Default|SetIsReversePatrol true)
                          (Variables|Default|SetCounter_PatrolArray (- _returnvalue 1)))))))))))
        (else
          (Development|PrintString "No Patrol Goals in Array" true true "(R=0.543750,G=0.000000,B=0.019312,A=1.000000)" 5.0)
          (Variables|Default|SetPatrolType "EPT_FullRandom"))))))

(fn InitializeMovementGoal
  (Variables|Default|SetStarting%20Location (Transformation|GetActorLocation))
  ;[1 1 1] Make Spawn Point
  (bind _returnvalue (Game|SpawnActorfromClass "/Game/Blueprints/BP_MovementGoalActor.BP_MovementGoalActor_C" (Transformation|GetActorTransform) "Undefined" 0 0))
  (Variables|Default|SetSpawnPoint _returnvalue))

(fn InverseMovementGoalLocation
  (Variables|Default|SetIsChangingDirection true)
  (Transformation|SetActorLocation (Variables|Default|GetMovement%20Goal) (Math|Transform|InverseTransformDirection (Transformation|GetActorTransform) (Transformation|GetVelocity)) false false))

(fn IfStationary,ChangeMovementGoal
  (bind _charactermovement (Variables|Character|GetCharacterMovement))
  (bind _returnvalue (Pawn|Components|CharacterMovement|GetLastUpdateVelocity _charactermovement))
  (if (not (Variables|Default|GetIsLoading))
    (if (<= (Math|Float|Absolute(Float) (.x _returnvalue)) 0.0)
      (if (<= (Math|Float|Absolute(Float) (.y _returnvalue)) 0.0)
        (if (<= (Math|Float|Absolute(Float) (.z _returnvalue)) 0.0)
          (Variables|Default|SetIsChangingDirection true)
          (CallFunction|SetNewMovementGoal))))))

(fn MovetoStartingLocation
  (Variables|Default|SetMovement%20Goal (Variables|Default|GetSpawnPoint))
  (CallFunction|IdleMovement))

(fn IfResetEndRegen
  (if (Utilities|Operators|EqualEqual (Variables|Default|GetStarting%20Location) (Transformation|GetActorLocation) 1e+01)
    (Variables|Default|SetIsChangingDirection true)
    (CallFunction|SetNewMovementGoal)
    (Variables|Default|SetIsReturning false)))

(fn SetWeapon
  (switch Utilities|FlowControl|Switch|SwitchonEWeaponType (Variables|Default|GetWeaponType)
    (:EWT_Sword
      (Variables|Default|SetAttackMontage "/Game/Blueprints/Enemy/Animations/WeaponAnimations/1h/AM_Alien1hAttacks.AM_Alien1hAttacks")
      (|Sword))
    (:EWT_GreatHammer
      (Variables|Default|SetAttackMontage "/Game/Blueprints/Enemy/Animations/WeaponAnimations/2h/AM_Alien2hAttacks.AM_Alien2hAttacks")
      (|Hammer))
    (:EWT_Rifle
      (Variables|Default|SetAttackMontage "/Game/Blueprints/Enemy/Animations/WeaponAnimations/rifle/AM_AlienRifleAttacks.AM_AlienRifleAttacks")
      (Variables|Default|SetHasRangedWeapon true)
      (|Rifle))
    (:EWT_Pistol
      (Variables|Default|SetAttackMontage "/Game/Blueprints/Enemy/Animations/WeaponAnimations/pistol/AM_AlienPistolAttacks.AM_AlienPistolAttacks")
      (Variables|Default|SetHasRangedWeapon true)
      (|Pistol))
    (:EWT_Bow
      (Variables|Default|SetAttackMontage "/Game/Blueprints/Enemy/Animations/WeaponAnimations/bow/AM_AlienBowAttacks.AM_AlienBowAttacks")
      (Variables|Default|SetHasRangedWeapon true)
      (|Bow))))

(event Custom|OnSeePawn_Event
  (params (Pawn :type Pawn%20Object%20Reference))
  (bind _asbp_slash_character (Utilities|Casting|CastToBP_SlashCharacter Pawn))
  (Variables|Default|SetIsInCombat true)
  (Variables|Default|SetCombatTarget _asbp_slash_character)
  (Variables|Default|SetIsChangingDirection false)
  (Variables|/Script/Engine.CharacterMovementComponent|SetMaxWalkSpeed (Variables|Character|GetCharacterMovement) 4e+02)
  (CallFunction|PursuePlayerifinCombat))

(event Custom|OnHearNoise_Event
  (params (Instigator :type Pawn%20Object%20Reference) (Location :type Vector%20%28by%20ref%29) (Volume :type Float%20%28single-precision%29))
  (bind _asbp_slash_character (Utilities|Casting|CastToBP_SlashCharacter Instigator))
  (Variables|Default|SetIsInCombat true)
  (Variables|Default|SetCombatTarget _asbp_slash_character)
  (Variables|Default|SetIsChangingDirection false)
  (Variables|/Script/Engine.CharacterMovementComponent|SetMaxWalkSpeed (Variables|Character|GetCharacterMovement) 4e+02)
  (CallFunction|PursuePlayerifinCombat))